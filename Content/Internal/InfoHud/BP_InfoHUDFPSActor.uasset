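; Actor that adds the UMG_InfoHUD widget to the game's main HUD when play begins.
; It casts the local player controller's HUD to BP_HUD, creates the widget and attaches it to the main widget's MainCanvas, anchored to stretch across the canvas.
; It logs whether the HUD was found and has no other active logic.
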(event `self.ReceiveBeginPlay`
  (bind _asbp_hud (cast `/Game/00_Main/Core/HUD/BP_HUD` (`PlayerController.GetHUD` (`IGS_BlueprintUtilities.GetLocalPlayerController` self)))
    (:`then`
      (bind _returnvalue (`|CreateWidget` "/NewAdventures/Internal/InfoHud/UI/UMG_InfoHUD.UMG_InfoHUD_C"))
      (bind _returnvalue_2 (`CanvasPanel.AddChildToCanvas` (`IGS_MainHUDWidget.MainCanvas` (`IGS_MainHUD.MainHUDWidget` _asbp_hud)) _returnvalue))
      (`CanvasPanelSlot.SetLayout` _returnvalue_2 (make `AnchorData` (make `Margin` 0.0) (make `Anchors` (0.0 0.0) (1.0 1.0))))
      (`self.Log` "Added HUD"))
    (:`CastFailed`
      (`self.Log` "Failed to find HUD" "NewEnumerator4"))))

(fn `UserConstructionScript`
  (`parent.UserConstructionScript`))