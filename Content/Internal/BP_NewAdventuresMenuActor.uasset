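; Menu actor for the New Adventures mod that injects mod missions and settings into the game's menus.
; On BeginPlay it adds a mission category to any existing multiplayer jobs screen and listens for screen opens.
; Clicking a mod mission creates a multiplayer lobby with fixed difficulty and heat.
; Opening Options inserts a settings tab and submenu by rebuilding the tab row, guarded by a hardcoded tab count.
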(event `DebugLogScreenHandler`
  (bind _returnvalue (subsystem `IGS_ScreenHandler`))
  (add `IGS_ScreenHandler.OnScreenOpenWithTag` _returnvalue (delegate `DebugOnScreenOpenWithTag`))
  (add `IGS_ScreenHandler.OnScreenSwitched` _returnvalue (delegate `DebugOnScreenSwitched`)))

(event `self.ReceiveBeginPlay`
  (`|ExecutionSequence`
    (:`then_0`
      (add `IGS_ScreenHandler.OnScreenOpenWithTag` (subsystem `IGS_ScreenHandler`) (`|CreateDelegate` :!event `OnScreenOpenWithTag`)))
    (:`then_1`
      (bind _foundwidgets (`WidgetBlueprintLibrary.GetAllWidgetsOfClass` "/Game/00_Main/UI/Multiplayer/UMG_Multiplayer_JobsScreen.UMG_Multiplayer_JobsScreen_C" false))
      (if (not (== (`KismetArrayLibrary.Array_Length` _foundwidgets) 0))
        (bind _output (`|GetArrayItem` _foundwidgets))
        (`self.HookJobsScreen` _output)
        (`/NewAdventures/NA_Mod.Log` (`self.Mod`) (`|FormatText` "Hook jobs <Path>{0}</>" (`KismetSystemLibrary.GetPathName` _output)) "NewEnumerator0")))))

(event `DebugOnScreenOpenWithTag`
  (params (screenTag :type "GameplayTag Structure"))
  (`/NewAdventures/NA_Mod.Log` (`self.Mod`) (`|FormatText` "Open screen with tag <Arg>{0}</>" (`BlueprintGameplayTagLibrary.GetTagName` screenTag)) "NewEnumerator0"))

(event `DebugOnScreenSwitched`
  (params (screenTag :type "GameplayTag Structure"))
  (`/NewAdventures/NA_Mod.Log` (`self.Mod`) (`|FormatText` "Switch to screen <Arg>{0}</>" (`BlueprintGameplayTagLibrary.GetTagName` screenTag)) "NewEnumerator0"))

(event `HookJobsScreen`
  (params (Screen :type "/Game/00_Main/UI/Multiplayer/UMG_Multiplayer_JobsScreen Object Reference"))
  (bind _jobscategoriescontent (`IGS_JobsScreen.JobsCategoriesContent` Screen))
  (`/Engine/EditorBlueprintResources/StandardMacros.IsValid` (`self.ModJobsCategory`)
    (:`Is Not Valid`
      (set `self.JobsScreen` Screen)
      (bind _returnvalue (`|CreateWidget` "/NewAdventures/Internal/UI/Jobs/UMG_ModJobsCategory.UMG_ModJobsCategory_C" (`Widget.GetOwningPlayer` _jobscategoriescontent)))
      (bind _output_get (set `self.ModJobsCategory` _returnvalue))
      (bind _returnvalue_2 (`/NewAdventures/Internal/BPFL_Internal.FindAllMissons`))
      (`/NewAdventures/Internal/UI/Jobs/UMG_ModJobsCategory.SetMissions` _output_get _returnvalue_2)
      (add `/NewAdventures/Internal/UI/Jobs/UMG_ModJobsCategory.OnJobItemSelected` _output_get (delegate `OnJobItemSelected`))
      (add `/NewAdventures/Internal/UI/Jobs/UMG_ModJobsCategory.OnMissionClicked` _output_get (delegate `OnMissionClicked`))
      (`PanelWidget.AddChild` _jobscategoriescontent _output_get))))

(event `HookSettingsMenu`
  (params (Screen :type "/Game/00_Main/Core/UI/Menus/Settings/UMG_SettingsMenu Object Reference"))
  (bind _returnvalue (`Widget.GetOwningPlayer` Screen))
  (bind _tabsonly (`/Game/00_Main/Core/UI/Menus/Settings/UMG_SettingsMenu.TabsOnly` Screen))
  (if (== (`PanelWidget.GetChildrenCount` (`/Game/00_Main/Core/UI/Menus/Settings/UMG_SettingsMenu.TabsOnly` Screen)) 11)
    (`|ExecutionSequence`
      (:`then_0`
        (`|ExecutionSequence`
          (:`then_0`
            (set `self.TabsOnlyChildren` (`PanelWidget.GetAllChildren` _tabsonly)))
          (:`then_1`
            (bind _returnvalue_2 (`|CreateWidget` "/NewAdventures/Internal/UI/UMG_SettingsTabsEXT.UMG_SettingsTabsEXT_C" _returnvalue))
            (`KismetArrayLibrary.Array_Insert` (`self.TabsOnlyChildren`) _returnvalue_2 9))
          (:`then_2`
            (for _array_element (`self.TabsOnlyChildren`)
              (`HorizontalBox.AddChildToHorizontalBox` _tabsonly _array_element)))))
      (:`then_1`
        (`|ExecutionSequence`
          (:`then_0`
            (bind _returnvalue_3 (`|CreateWidget` "/NewAdventures/Internal/UI/UMG_ModSettingsSubmenu.UMG_ModSettingsSubmenu_C" _returnvalue))
            (`PanelWidget.AddChild` (`IGS_WidgetOptionsMenu.SettingsWidgetSwitcher` Screen) _returnvalue_3))))
      (:`then_2`
        (`/NewAdventures/NA_Mod.Log` (`self.Mod`) (`|FormatText` "Hooked settings menu <Path>{0}</>" Screen) "NewEnumerator0")))))

(event `OnMissionClicked`
  (params (Mission :type "/NewAdventures/Internal/BP_MissionInfo Object Reference"))
  (`/NewAdventures/Internal/BP_NewAdventuresMod.CreateMultiplayerLobbyForModMission` (`self.NANewAdventures`) Mission "SD_MediumForce" "Medium"))

(event `OnJobItemSelected`
  (params (JobWidget :type "IGS_JobsItemWidget Object Reference"))
  (`/Game/00_Main/UI/Multiplayer/UMG_Multiplayer_JobsScreen.OnJobItemSelectionChanged` (`self.JobsScreen`) (cast `/Game/00_Main/UI/Multiplayer/UMG_JobsItem` JobWidget :!pure true)))

(event `OnScreenOpenWithTag`
  (params (ScreenTag :type "GameplayTag Structure"))
  (`|ExecutionSequence`
    (:`then_0`
      (if (`BlueprintGameplayTagLibrary.MatchesTag` ScreenTag (struct :`TagName` "MainMenu.Options"))
        (`self.HookSettingsMenu` (cast `/Game/00_Main/Core/UI/Menus/Settings/UMG_SettingsMenu` (`IGS_ScreenHandler.GetOpenedScreenByTag` (subsystem `IGS_ScreenHandler`) (struct :`TagName` "MainMenu.Options")) :!pure true))))))

(fn `UserConstructionScript`
  (`parent.UserConstructionScript`))