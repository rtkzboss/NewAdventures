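; BP_MissionInfo is a mission information object that exposes the descriptive details of a mission.
; Three getter functions return the Name, Image and ShortDescription fields of its Data variable.
; Each getter passes its field through unchanged, with no other logic.
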(fn `GetImage`
  (returns (ReturnValue :type "Texture2D Soft Object Reference"))
  (return (`.Image_8_1AB3CD554005384579C212A8E19C0FE7` (break `/NewAdventures/NA_Mission` (`self.Data`)))))

(fn `GetName`
  (returns (ReturnValue :type Text))
  (return (`.Name_5_3D0D9BF84FC3458995BA8F82E3987007` (break `/NewAdventures/NA_Mission` (`self.Data`)))))

(fn `GetShortDescription`
  (returns (ReturnValue :type Text))
  (return (`.ShortDescription_11_820668ED48A087A32AA953942EC9E531` (break `/NewAdventures/NA_Mission` (`self.Data`)))))