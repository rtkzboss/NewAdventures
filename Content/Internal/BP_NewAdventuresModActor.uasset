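; In-game actor for the NewAdventures mod that manages its overlay and injects mod UI into the game's own screens.
; On BeginPlay it creates the overlay, forwards key presses to the mod and listens to IGSScreenHandler screen events.
; Opening Options triggers insertion of a mod settings tab and submenu, guarded by a hardcoded tab count.
; Any jobs screen found at BeginPlay gets a mod category filled from FindAllMissons.
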(event `self.ReceiveBeginPlay`
  (bind _returnvalue (subsystem `IGS_ScreenHandler`))
  (`|ExecutionSequence`
    (:`then_0`
      (set `self.NewAdventures` (cast `/NewAdventures/Internal/BP_NewAdventuresMod` (`self.Mod`) :!pure true))
      (`self.CreateOverlay`))
    (:`then_1`
      (`self.EnableInput` (`IGS_BlueprintUtilities.GetLocalPlayerController` self)))
    (:`then_2`
      (add `IGS_ScreenHandler.OnScreenOpenWithTag` _returnvalue (`|CreateDelegate` :!event `OnScreenOpenWithTag`))
      (add `IGS_ScreenHandler.OnScreenSwitched` _returnvalue (delegate `CustomEvent_0`)))
    (:`then_3`
      (bind _foundwidgets (`WidgetBlueprintLibrary.GetAllWidgetsOfClass` "/Game/00_Main/UI/Multiplayer/UMG_Multiplayer_JobsScreen.UMG_Multiplayer_JobsScreen_C" false))
      (if (not (== (`KismetArrayLibrary.Array_Length` _foundwidgets) 0))
        (bind _output (`|GetArrayItem` _foundwidgets))
        (`self.HookJobsScreen` _output)
        (`/NewAdventures/NA_Mod.Log` (`self.NewAdventures`) (`|FormatText` "Hook jobs {0}" (`KismetSystemLibrary.GetPathName` _output)) "NewEnumerator2")))))

(event `CustomEvent_0`
  (params (screenTag :type "GameplayTag Structure"))
  (`/NewAdventures/NA_Mod.Log` (`self.NewAdventures`) (`|FormatText` "Switch to screen <Arg>{0}</>" (`BlueprintGameplayTagLibrary.GetTagName` screenTag)) "NewEnumerator0"))

(event `Key|AnyKey` :consume false
  (params (Key :type "Key Structure"))
  (:`Pressed`
    (`/NewAdventures/Internal/BP_NewAdventuresMod.KeyPressed` (`self.NewAdventures`) Key)))

(fn `CreateOverlay`
  (`/Engine/EditorBlueprintResources/StandardMacros.IsValid` (`self.Overlay`)
    (:`Is Not Valid`
      (bind _returnvalue (`|CreateWidget` "/NewAdventures/Internal/UI/UMG_Overlay.UMG_Overlay_C" (`IGS_BlueprintUtilities.GetLocalPlayerController` self) (`self.NewAdventures`)))
      (bind _output_get (set `self.Overlay` _returnvalue))
      (`UserWidget.AddToViewport` _output_get 99999999))))

(fn `HookJobsScreen`
  (params (Screen :type "/Game/00_Main/UI/Multiplayer/UMG_Multiplayer_JobsScreen Object Reference"))
  (bind _jobscategoriescontent (`IGS_JobsScreen.JobsCategoriesContent` Screen))
  (`/Engine/EditorBlueprintResources/StandardMacros.IsValid` (`self.ModJobsCategory`)
    (:`Is Not Valid`
      (bind _returnvalue (`|CreateWidget` "/NewAdventures/Internal/UI/Jobs/UMG_ModJobsCategory.UMG_ModJobsCategory_C" (`Widget.GetOwningPlayer` _jobscategoriescontent)))
      (bind _output_get (set `self.ModJobsCategory` _returnvalue))
      (bind _returnvalue_2 (`/NewAdventures/Internal/BPFL_Internal.FindAllMissons`))
      (`/NewAdventures/Internal/UI/Jobs/UMG_ModJobsCategory.SetMissions` _output_get _returnvalue_2)
      (`PanelWidget.AddChild` _jobscategoriescontent _output_get))))

(fn `HookSettingsMenu`
  (params (Screen :type "/Game/00_Main/Core/UI/Menus/Settings/UMG_SettingsMenu Object Reference"))
  (locals (TabsOnlyChildren :type "Array of Widget Object Reference"))
  (bind _returnvalue (`Widget.GetOwningPlayer` Screen))
  (bind _tabsonly (`/Game/00_Main/Core/UI/Menus/Settings/UMG_SettingsMenu.TabsOnly` Screen))
  (if (== (`PanelWidget.GetChildrenCount` (`/Game/00_Main/Core/UI/Menus/Settings/UMG_SettingsMenu.TabsOnly` Screen)) 11)
    (`|ExecutionSequence`
      (:`then_0`
        (`|ExecutionSequence`
          (:`then_0`
            (set `local.TabsOnlyChildren` (`PanelWidget.GetAllChildren` _tabsonly)))
          (:`then_1`
            (bind _returnvalue_2 (`|CreateWidget` "/NewAdventures/Internal/UI/UMG_SettingsTabsEXT.UMG_SettingsTabsEXT_C" _returnvalue))
            (`KismetArrayLibrary.Array_Insert` (`local.TabsOnlyChildren`) _returnvalue_2 9))
          (:`then_2`
            (for _array_element (`local.TabsOnlyChildren`)
              (`HorizontalBox.AddChildToHorizontalBox` _tabsonly _array_element)))))
      (:`then_1`
        (`|ExecutionSequence`
          (:`then_0`
            (bind _returnvalue_3 (`|CreateWidget` "/NewAdventures/Internal/UI/UMG_ModSettingsSubmenu.UMG_ModSettingsSubmenu_C" _returnvalue))
            (`PanelWidget.AddChild` (`IGS_WidgetOptionsMenu.SettingsWidgetSwitcher` Screen) _returnvalue_3))))
      (:`then_2`
        (`/NewAdventures/NA_Mod.Log` (`self.NewAdventures`) (`|FormatText` "Hooked settings menu {0}" Screen) "NewEnumerator2")))))

(fn `OnScreenOpenWithTag`
  (params (ScreenTag :type "GameplayTag Structure"))
  (`|ExecutionSequence`
    (:`then_0`
      (if (`BlueprintGameplayTagLibrary.MatchesTag` ScreenTag (struct :`TagName` "MainMenu.Options"))
        (`self.HookSettingsMenu` (cast `/Game/00_Main/Core/UI/Menus/Settings/UMG_SettingsMenu` (`IGS_ScreenHandler.GetOpenedScreenByTag` (subsystem `IGS_ScreenHandler`) (struct :`TagName` "MainMenu.Options")) :!pure true))))
    (:`then_1`
      (`/NewAdventures/NA_Mod.Log` (`self.NewAdventures`) (`|FormatText` "Open screen {0}" (`BlueprintGameplayTagLibrary.GetTagName` ScreenTag)) "NewEnumerator0"))))

(fn `OpenOverlay`
  (`self.CreateOverlay`)
  (`/NewAdventures/Internal/UI/UMG_Overlay.Open` (`self.Overlay`)))

(fn `ToggleOverlay`
  (`self.CreateOverlay`)
  (`/NewAdventures/Internal/UI/UMG_Overlay.ToggleOpen` (`self.Overlay`)))

(fn `UserConstructionScript`
  (`parent.UserConstructionScript`))