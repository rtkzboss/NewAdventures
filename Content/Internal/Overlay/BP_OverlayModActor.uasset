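; BP_OverlayModActor is a mod actor that owns the overlay UI and exposes events to open, open for a command, toggle and close it.
; On BeginPlay it creates UMG_OverlayRoot for the local player controller, passes in the NewAdventures reference and adds it at a very high viewport Z-order.
; Open and toggle events recreate the widget if it is invalid before forwarding the call, while close acts only on a valid widget.
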(event `self.ReceiveBeginPlay`
  (`self.CreateOverlay`))

(event `CreateOverlay`
  (`/Engine/EditorBlueprintResources/StandardMacros.IsValid` (`self.OverlayRoot`)
    (:`Is Not Valid`
      (bind _returnvalue (`|CreateWidget` "/NewAdventures/Internal/Overlay/UI/UMG_OverlayRoot.UMG_OverlayRoot_C" (`IGS_BlueprintUtilities.GetLocalPlayerController` self) (`self.NANewAdventures`)))
      (bind _output_get (set `self.OverlayRoot` _returnvalue))
      (`UserWidget.AddToViewport` _output_get 99999999))))

(event `OpenOverlay`
  (`self.CreateOverlay`)
  (`/NewAdventures/Internal/Overlay/UI/UMG_OverlayRoot.Open` (`self.OverlayRoot`)))

(event `OpenOverlayForCommand`
  (`self.CreateOverlay`)
  (`/NewAdventures/Internal/Overlay/UI/UMG_OverlayRoot.OpenForCommand` (`self.OverlayRoot`)))

(event `ToggleOverlay`
  (`self.CreateOverlay`)
  (`/NewAdventures/Internal/Overlay/UI/UMG_OverlayRoot.ToggleOpen` (`self.OverlayRoot`)))

(event `CloseOverlay`
  (bind _overlayroot (`self.OverlayRoot`))
  (`/Engine/EditorBlueprintResources/StandardMacros.IsValid` _overlayroot
    (:`Is Valid`
      (`/NewAdventures/Internal/Overlay/UI/UMG_OverlayRoot.Close` _overlayroot))))

(fn `UserConstructionScript`
  (`parent.UserConstructionScript`))