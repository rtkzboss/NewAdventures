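; Internal mod Blueprint that adds debug console commands for log spam testing, listing key bindings and listing mods.
; OnCommand matches the command name, parses arguments and logs a usage error when too many are given.
; Spam logs a numbered test line a given or default number of times.
; The show commands iterate NANewAdventures' bound-key and mod maps, logging each entry as rich text with syntax-highlighted commands or class paths.
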(event `self.OnCommand`
  (params (Name :type Name) (Args :type String))
  (switch `name` Name
    (:`Spam`
      (bind (_arg _rest) (`/NewAdventures/Internal/BPML_Mod.ParseNextArg` Args)
        (:`Done`
          (`self.DebugSpamLog` 1000))
        (:`GotArg`
          (`/NewAdventures/Internal/BPML_Mod.ParseNextArg` _rest
            (:`Done`
              (`self.DebugSpamLog` (`KismetStringLibrary.Conv_StringToInt` _arg)))
            (:`GotArg`
              (`self.Log` (`/NewAdventures/Internal/BPFL_Internal.MakeCommandUsageString` Name "command-toomanyargs") "NewEnumerator4" :!label _label))))))
    (:`ShowBindings`
      (`/NewAdventures/Internal/BPML_Mod.ParseNextArg` Args
        (:`Done`
          (`self.DumpBoundKeys`))
        (:`GotArg`
          (goto _label))))
    (:`ShowMods`
      (`/NewAdventures/Internal/BPML_Mod.ParseNextArg` Args
        (:`Done`
          (`self.DumpMods`))
        (:`GotArg`
          (goto _label))))))

(event `DebugSpamLog`
  (params (N :type Integer))
  (for _index (range 1 (+ N 1))
    (`self.Log` (`|FormatText` "Testing log performance <Arg>{0}</>/<Arg>{1}</>" _index N) "NewEnumerator0")))

(event `DumpBoundKeys`
  (bind _boundkeys (`/NewAdventures/Internal/BP_NewAdventuresMod.BoundKeys` (`self.NANewAdventures`)))
  (bind _keys (`BlueprintMapLibrary.Map_Keys` _boundkeys))
  (for _array_element _keys
    (bind (_modobject _name _command) (break `/NewAdventures/Internal/S_BoundKey` (`BlueprintMapLibrary.Map_Find` _boundkeys _array_element)))
    (bind _text (`/NewAdventures/Internal/BPFL_Internal.SyntaxHighlightCommand_Compatible` _command))
    (`/Engine/EditorBlueprintResources/StandardMacros.IsValid` _modobject
      (:`Is Valid`
        (bind _returnvalue (`self.GetName` _modobject))
        (bind _returnvalue_2 (`KismetInputLibrary.Key_GetDisplayName` _array_element))
        (`self.Log` (`|FormatText` "<Key>{Key}</> → <Arg>{Name}</> in <Mod>{Mod}</> = {Command}" _returnvalue_2 _name _returnvalue _text)))
      (:`Is Not Valid`
        (`self.Log` (`|FormatText` "<Key>{Key}</> → <Arg>{Name}</Arg> = {Command}" _returnvalue_2 _name _text))))))

(event `DumpMods`
  (bind _modsbyinternalname (`/NewAdventures/Internal/BP_NewAdventuresMod.ModsByInternalName` (`self.NANewAdventures`)))
  (bind _keys (`BlueprintMapLibrary.Map_Keys` _modsbyinternalname))
  (bind _values (`BlueprintMapLibrary.Map_Values` _modsbyinternalname))
  (for (_array_element _array_index) _keys
    (`|ExecutionSequence`
      (:`then_0`
        (bind _output (`|GetArrayItem` _values _array_index))
        (bind _returnvalue (`self.GetName` _output)))
      (:`then_2`
        (`self.Log` (`|FormatText` "<Mod>{Name}</>: <Arg>{InternalName}</> at <Path>{Path}</>" _returnvalue _array_element (`/NewAdventures/Internal/BPFL_Internal.GetPathName` (`GameplayStatics.GetObjectClass` _output))))))))