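; Central manager for the New Adventures mod framework, discovering NA mods and running them across level transitions.
; Level-load events preload each mod's actor classes asynchronously, and state changes spawn its general actor plus a menu or FPS variant.
; Key presses call mod functions by name through bindings built from mod defaults.
; Also provides a filtered log with unseen counts, debug tracing and multiplayer lobby creation for mod missions via debug job data.
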(event `self.Init`
  (bind _returnvalue (subsystem `IGS_LevelTransitionManager`))
  (`|ExecutionSequence`
    (:`then_0`
      (bind _returnvalue_2 (`/NewAdventures/Internal/BPFL_Internal.FindAllNAMods`))
      (set `self.NAMods` _returnvalue_2))
    (:`then_1`
      (add `IGS_LevelTransitionManager.OnLevelTransitionStateChangeStarted` _returnvalue (`|CreateDelegate` :!event `OnLevelTransitionStateChanged`))
      (add `IGS_LevelTransitionManager.OnLevelLoadStarted` _returnvalue (`|CreateDelegate` :!event `OnLevelLoadStarted`)))
    (:`then_2`
      (`self.UpdateKeyBindings`))
    (:`then_3`
      (`self.DebugLogDiscovery`)
      (`self.DebugBindLevelTransitionManager`))))

(event `DebugBindLevelTransitionManager`
  (bind _returnvalue (subsystem `IGS_LevelTransitionManager`))
  (add `IGS_LevelTransitionManager.OnLevelLoadStarted` _returnvalue (delegate `DebugOnLevelLoadStarted`))
  (add `IGS_LevelTransitionManager.OnLevelLoadInterrupted` _returnvalue (delegate `DebugOnLevelLoadInterrupted`))
  (add `IGS_LevelTransitionManager.OnLevelLoadFinished` _returnvalue (delegate `DebugOnLevelLoadFinished`))
  (add `IGS_LevelTransitionManager.OnLevelLoadAttemptSuccess` _returnvalue (delegate `DebugOnLevelLoadAttemptSuccess`))
  (add `IGS_LevelTransitionManager.OnLevelLoadAttemptFailure` _returnvalue (delegate `DebugOnLevelLoadAttemptFailure`))
  (add `IGS_LevelTransitionManager.OnLevelTransitionStateChangeStarted` _returnvalue (delegate `DebugOnLevelTransitionStateChangeStarted`))
  (add `IGS_LevelTransitionManager.OnLevelTransitionStateChanged` _returnvalue (delegate `DebugOnLevelTransitionStateChanged`)))

(event `DebugOnLevelLoadStarted`
  (params (inLevelName :type Name) (inIsServerTravel :type Boolean))
  (`self.Log` (`|FormatText` "Level load started <Arg>{0}</> is server travel=<Arg>{1}</> gamestate=<Arg>{2}</>" inLevelName inIsServerTravel (`KismetSystemLibrary.GetPathName` (`GameplayStatics.GetGameState`))) "NewEnumerator0"))

(event `DebugOnLevelLoadInterrupted`
  (params (inLevelName :type Name) (inIsServerTravel :type Boolean))
  (`self.Log` (`|FormatText` "Level load interrupted <Arg>{0}</> is server travel=<Arg>{1}</> gamestate=<Arg>{2}</>" inLevelName inIsServerTravel (`KismetSystemLibrary.GetPathName` (`GameplayStatics.GetGameState`))) "NewEnumerator0"))

(event `DebugOnLevelLoadFinished`
  (params (inLevelName :type Name) (inIsServerTravel :type Boolean))
  (`self.Log` (`|FormatText` "Level load finished <Arg>{0}</> is server travel=<Arg>{1}</> gamestate=<Arg>{2}</>" inLevelName inIsServerTravel (`KismetSystemLibrary.GetPathName` (`GameplayStatics.GetGameState`))) "NewEnumerator0"))

(event `UpdateKeyBindings`
  (`BlueprintMapLibrary.Map_Clear` (`self.KeyBindings`))
  (for _array_element (`self.NAMods`)
    (for _array_element_2 (`/NewAdventures/NA_Mod.Bindings` _array_element)
      (bind (_name _event _defaultkey) (break `/NewAdventures/NA_Binding` _array_element_2))
      (`BlueprintMapLibrary.Map_Add` (`self.KeyBindings`) _defaultkey (make `/NewAdventures/Internal/S_BoundKey` _array_element _event)))))

(event `DebugOnLevelLoadAttemptSuccess`
  (params (inLevelName :type Name) (inIsServerTravel :type Boolean))
  (`self.Log` (`|FormatText` "Level load attempt success <Arg>{0}</> is server travel=<Arg>{1}</> gamestate=<Arg>{2}</>" inLevelName inIsServerTravel (`KismetSystemLibrary.GetPathName` (`GameplayStatics.GetGameState`))) "NewEnumerator0"))

(event `DebugOnLevelLoadAttemptFailure`
  (params (inLevelName :type Name) (inIsServerTravel :type Boolean))
  (`self.Log` (`|FormatText` "Level load attempt failure <Arg>{0}</> is server travel=<Arg>{1}</> gamestate=<Arg>{2}</>" inLevelName inIsServerTravel (`KismetSystemLibrary.GetPathName` (`GameplayStatics.GetGameState`))) "NewEnumerator0"))

(event `PreloadActor`
  (params (Class :type "/NewAdventures/NA_ModActor Soft Class Reference (by ref)"))
  (if (`KismetSystemLibrary.IsValidSoftClassReference` Class)
    (`|ExecutionSequence`
      (:`then_0`
        (bind _class (`|LoadAssetClass` Class)
          (:`Completed`
            (`KismetArrayLibrary.Array_Add` (`self.NAPreloadedActorClasses`) _class))))
      (:`then_1`
        (`self.Log` (`|FormatText` "Preload {0}" (`KismetSystemLibrary.Conv_SoftClassReferenceToString` Class)) "NewEnumerator0")))))

(event `DebugOnLevelTransitionStateChangeStarted`
  (params (inCurrentState :type "EIGS_LevelTransitionType Enum" :default "LT_Unknown") (inPreviousState :type "EIGS_LevelTransitionType Enum" :default "LT_Unknown"))
  (`self.Log` (`|FormatText` "Level load state change started <Arg>{1}</> -> <Arg>{0}</> gamestate=<Arg>{2}</>" (`|GetEnumeratorNameAsString` inPreviousState) (`|GetEnumeratorNameAsString` inCurrentState) (`KismetSystemLibrary.GetPathName` (`GameplayStatics.GetGameState`))) "NewEnumerator0"))

(event `DebugOnLevelTransitionStateChanged`
  (params (inCurrentState :type "EIGS_LevelTransitionType Enum" :default "LT_Unknown") (inPreviousState :type "EIGS_LevelTransitionType Enum" :default "LT_Unknown"))
  (`self.Log` (`|FormatText` "Level load state changed <Arg>{1}</> -> <Arg>{0}</> gamestate=<Arg>{2}</>" (`|GetEnumeratorNameAsString` inPreviousState) (`|GetEnumeratorNameAsString` inCurrentState) (`KismetSystemLibrary.GetPathName` (`GameplayStatics.GetGameState`))) "NewEnumerator0"))

(event `DebugLogDiscovery`
  (`|ExecutionSequence`
    (:`then_0`
      (bind _returnvalue (`/NewAdventures/Internal/BPFL_Internal.GetSortedModInfos`))
      (for _array_element _returnvalue
        (`self.Log` (`|FormatText` "Found mod <Arg>{0}</> in <Arg>{1}</>" (`/NewAdventures/Internal/UI/BP_ModInfo.Name` _array_element) (`/NewAdventures/Internal/UI/BP_ModInfo.MountPoint` _array_element)) "NewEnumerator0")))
    (:`then_1`
      (bind _returnvalue_2 (`/NewAdventures/Internal/BPFL_Internal.FindAllMissons`))
      (for _array_element_2 _returnvalue_2
        (`self.Log` (`|FormatText` "Found mission <Arg>{0}</>" (`.Name_5_3D0D9BF84FC3458995BA8F82E3987007` (break `/NewAdventures/NA_Mission` (`/NewAdventures/Internal/BP_MissionInfo.Data` _array_element_2)))) "NewEnumerator0")))))

(event `DebugSpamLog`
  (params (N :type Integer))
  (for _index (range 1 (+ N 1))
    (`self.Log` (`|FormatText` "Testing log performance <Arg>{0}</>/<Arg>{1}</>" _index N) "NewEnumerator0")))

(fn `AddItemToLog`
  (params (Item :type "/NewAdventures/NA_LogItem Object Reference"))
  (bind _level (`/NewAdventures/NA_LogItem.Level` Item))
  (if (>= _level (`self.LogFilter`))
    (`|ExecutionSequence`
      (:`then_0`
        (`self.IncrLogUnseen` _level))
      (:`then_1`
        (`KismetArrayLibrary.Array_Add` (`self.LogItems`) Item)
        (`self.OnLog` Item)
        (`KismetSystemLibrary.PrintString` (`KismetTextLibrary.Conv_TextToString` (`/NewAdventures/NA_LogItem.Message` Item)) true true (struct :`R` 0.991858 :`B` 1.0 :`A` 1.0))))))

(fn `AddToLog`
  (params (Mod :type "/NewAdventures/NA_IMod Interface") (Level :type "/NewAdventures/NA_LogLevel Enum" :default "NewEnumerator0") (Message :type Text))
  (bind _returnvalue (`|GenericCreateObject` "/NewAdventures/NA_LogItem.NA_LogItem_C" self Mod Level Message (`KismetMathLibrary.Now`)))
  (`self.AddItemToLog` _returnvalue))

(fn `CreateMultiplayerLobbyForModMission`
  (params (Mission :type "/NewAdventures/Internal/BP_MissionInfo Object Reference") (ScenarioDifficulty :type "EIGS_ScenarioDifficulty Enum" :default "SD_Unknown") (Heat :type "EMETA_Heat Enum" :default "INVALID"))
  (bind (_name _shortdescription _mainobjective _longdescription _image _map _fpsmissionid) (break `/NewAdventures/NA_Mission` (`/NewAdventures/Internal/BP_MissionInfo.Data` Mission)))
  (`self.RequestMultiplayerMissionLobby` (make `IGS_Meta2FPS_Data` (struct :`TagName` "Mission.Unknown") (`KismetStringLibrary.Conv_NameToString` _map) (struct :`TagName` "Mission.Unknown") "None" "Downtown" "AllRandom" "Sunset" ScenarioDifficulty "FD_Normal" Heat 0 -1 (`BlueprintGameplayTagLibrary.MakeLiteralGameplayTag` (struct :`TagName` "MetaData.BonusObjective.ReviveUseMax1")) false "None" "INVALID" "" "INVALID" _name 0 0 -1 (struct) (struct) "Connected" false "Unknown" "US_None" "AT_Tier1" "US_Sicarios" "AT_Tier2" "US_SWAT" "AT_Tier2" "US_None" "AT_Tier2" -1 (struct) 50 false false -1 true) _fpsmissionid)
  (bind _asumg_multiplayer_menu_base (cast `/Game/00_Main/UI/Multiplayer/UMG_MultiplayerMenuBase` (`IGS_GameScreenHandler.GetBaseScreen` (subsystem `IGS_GameScreenHandler`))))
  (bind _missioninfo (`/Game/00_Main/UI/Multiplayer/UMG_Multiplayer_CreateLobbyScreen.MissionInfo` (`/Game/00_Main/UI/Multiplayer/UMG_MultiplayerMenuBase.UMG_Multiplayer_CreateLobbyScreen` _asumg_multiplayer_menu_base)))
  (`TextBlock.SetText` (`/Game/00_Main/UI/Multiplayer/UMG_MultiplayerMissionInfo.MissionName` _missioninfo) _name)
  (`TextBlock.SetText` (`/Game/00_Main/UI/Multiplayer/UMG_MultiplayerMissionInfo.MissionDescription` _missioninfo) _longdescription)
  (bind _mainobjective_2 (`/Game/00_Main/UI/Multiplayer/UMG_MultiplayerMissionInfo.MainObjective` _missioninfo))
  (`/Game/00_Main/Maps/Menu/UMG_MissionInfo_ObjectiveItem.SetAsMainObjective` _mainobjective_2 _mainobjective)
  (`Widget.SetVisibility` _mainobjective_2 "Visible")
  (`Widget.SetVisibility` (`/Game/00_Main/UI/Multiplayer/UMG_MultiplayerMissionInfo.SpecialObjective` _missioninfo) "Collapsed")
  (`Widget.SetVisibility` (`/Game/00_Main/UI/Multiplayer/UMG_MultiplayerMissionInfo.ExpectedValue` _missioninfo) "Collapsed")
  (`self.Log` "Done updating create lobby screen" "NewEnumerator0"))

(fn `IncrLogUnseen`
  (params (Level :type "/NewAdventures/NA_LogLevel Enum" :default "NewEnumerator0"))
  (bind _returnvalue (> (`self.LogUnseenCount`) 0))
  (if (>= Level (select `bool` _returnvalue :`false` (`self.LogUnseenFilter`) :`true` (`self.LogUnseenLevel`)))
    (if (and _returnvalue (`|EnumEquality` Level (`self.LogUnseenLevel`)))
      (`/Engine/EditorBlueprintResources/StandardMacros.IncrementInt` (`self.LogUnseenCount`)
        (:`  `
          _))
      (else
        (set `self.LogUnseenCount` 1)
        (set `self.LogUnseenLevel` Level)))
    (`self.OnLogUnseenChanged` (`self.LogUnseenLevel`) (`self.LogUnseenCount`))))

(fn `KeyPressed`
  (params (Key :type "Key Structure" :default "None"))
  (bind (_value _returnvalue) (`BlueprintMapLibrary.Map_Find` (`self.KeyBindings`) Key))
  (bind (_modobject _name) (break `/NewAdventures/Internal/S_BoundKey` _value))
  (if _returnvalue
    (`KismetSystemLibrary.K2_SetTimer` _modobject (`KismetStringLibrary.Conv_NameToString` _name))))

(fn `OnLevelLoadStarted`
  (params (inLevelName :type Name) (inIsServerTravel :type Boolean))
  (`self.PreloadActors` (`/NewAdventures/Internal/BPFL_Internal.IsMenuMap` inLevelName)))

(fn `OnLevelTransitionStateChanged`
  (params (inCurrentState :type "EIGS_LevelTransitionType Enum" :default "LT_Unknown") (inPreviousState :type "EIGS_LevelTransitionType Enum" :default "LT_Unknown"))
  (if (not (`|EnumEquality` inCurrentState "LT_Loading"))
    (`self.SpawnActors` (`.bSuccess` (cast `IGS_GameStateMenuBase` (`GameplayStatics.GetGameState`) :!pure true)))))

(fn `PreloadActors`
  (params (bIsMenu :type Boolean))
  (`KismetArrayLibrary.Array_Clear` (`self.PreloadedActorClasses`))
  (for _array_element (`self.NAMods`)
    (`self.PreloadActor` (`/NewAdventures/NA_Mod.ModActor` _array_element))
    (`self.PreloadActor` (select `bool` bIsMenu :`false` (`/NewAdventures/NA_Mod.FPSActor` _array_element) :`true` (`/NewAdventures/NA_Mod.MenuActor` _array_element) :!type "/NewAdventures/NA_ModActor Soft Class Reference"))))

(fn `RequestMultiplayerMissionLobby`
  (params (CustomMissionData :type "IGS_Meta2FPS_Data Structure") (FPSMissionID :type "IGS_BaseMissionObject Class Reference"))
  (bind ((`MissionTag` _missiontag) (`MapName` _mapname) (`MissionScenario` _missionscenario)) (break `IGS_Meta2FPS_Data` CustomMissionData))
  (`|ExecutionSequence`
    (:`then_0`
      (`self.Log` (`|FormatText` "Requesting multiplayer mission lobby for <Arg>{0}</>" _mapname) "NewEnumerator1"))
    (:`then_1`
      (bind _asbp_game_mode_menu (cast `/Game/00_Main/Core/GameModes/BP_GameMode_Menu` (`GameplayStatics.GetGameMode`)))
      (bind _asbp_game_state_quickplay_menu (cast `/Game/00_Main/Core/GameModes/BP_GameState_QuickplayMenu` (`GameplayStatics.GetGameState`)))
      (`|ExecutionSequence`
        (:`then_0`
          (bind _jobmanager (`/Game/00_Main/Core/GameModes/BP_GameState_QuickplayMenu.JobManager` _asbp_game_state_quickplay_menu))
          (`/Game/00_Main/Core/MainMenu/Managers/BP_quick_JobManagerComponent.DEBUG_SetCusomMissionData` _jobmanager CustomMissionData FPSMissionID)
          (`IGS_JobManagerBaseComponent.SetCurrentJob` _jobmanager null))
        (:`then_1`
          (`/Game/00_Main/Core/GameModes/BP_GameMode_Menu.RequestMissionLobby` _asbp_game_mode_menu null)
          (`/Game/00_Main/Core/GameModes/BP_GameMode_Menu.SetLobbyStartupSource` _asbp_game_mode_menu "Debug"))
        (:`then_2`
          (`IGS_GameStateBaseWithData.SetMissionTag` _asbp_game_state_quickplay_menu _missiontag)
          (`IGS_GameStateBaseWithData.SetMissionScenario` _asbp_game_state_quickplay_menu _missionscenario))))))

(fn `ResetLogUnseen`
  (if (> (`self.LogUnseenCount`) 0)
    (set `self.LogUnseenCount` 0)
    (`self.OnLogUnseenChanged` (`self.LogUnseenFilter`))))

(fn `SpawnActor`
  (params (Class :type "/NewAdventures/NA_ModActor Soft Class Reference") (Mod :type "/NewAdventures/NA_Mod Object Reference"))
  (returns (Actor :type "/NewAdventures/NA_ModActor Object Reference"))
  (if (`KismetSystemLibrary.IsValidSoftClassReference` Class)
    (`|ExecutionSequence`
      (:`then_0`
        (bind _returnvalue (`KismetSystemLibrary.LoadClassAsset_Blocking` Class))
        (bind _returnvalue_2 (`|SpawnActorFromClass` (castclass `/NewAdventures/NA_ModActor` _returnvalue :!pure true) (`KismetMathLibrary.MakeTransform` (0.0 0.0 0.0)) "AlwaysSpawn" "OverrideRootScale" null Mod null)))
      (:`then_1`
        (`self.Log` (`|FormatText` "Spawn {0}" (`KismetSystemLibrary.Conv_SoftClassReferenceToString` Class)) "NewEnumerator0"))
      (:`then_2`
        (return _returnvalue_2)))))

(fn `SpawnActors`
  (params (bIsMenu :type Boolean))
  (`BlueprintMapLibrary.Map_Clear` (`self.ModActors`))
  (`BlueprintMapLibrary.Map_Clear` (`self.FPSActors`))
  (`BlueprintMapLibrary.Map_Clear` (`self.MenuActors`))
  (for _array_element (`self.NAMods`)
    (`|ExecutionSequence`
      (:`then_0`
        (bind _actor (`self.SpawnActor` (`/NewAdventures/NA_Mod.ModActor` _array_element) _array_element))
        (`BlueprintMapLibrary.Map_Add` (`self.ModActors`) _array_element _actor))
      (:`then_1`
        (if bIsMenu
          (bind _actor_2 (`self.SpawnActor` (`/NewAdventures/NA_Mod.MenuActor` _array_element) _array_element))
          (`BlueprintMapLibrary.Map_Add` (`self.MenuActors`) _array_element (cast `/NewAdventures/NA_MenuActor` _actor_2 :!pure true))
          (else
            (bind _actor_3 (`self.SpawnActor` (`/NewAdventures/NA_Mod.FPSActor` _array_element)))
            (`BlueprintMapLibrary.Map_Add` (`self.FPSActors`) _array_element (cast `/NewAdventures/NA_FPSActor` _actor_3 :!pure true))))))))

(fn `ToggleOverlay`
  (bind _asbp_new_adventures_mod_actor (cast `/NewAdventures/Internal/BP_NewAdventuresModActor` (`self.GetModActor`)))
  (`/NewAdventures/Internal/BP_NewAdventuresModActor.ToggleOverlay` _asbp_new_adventures_mod_actor))